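; Multiplayer player character with team-colored armor and eyes, a class-specific weapon and melee combat.
; Attack input runs a cooldown-gated server-to-multicast swing, where a timeline rotates the weapon attachment point and only authority enables the weapon's box hitbox.
; Damage lowers health held in the PlayerState, which also supplies class damage; GetCurrentHealth is a stub returning zero.
; Death multicasts a ragdoll, then after a delay respawns through the player controller and destroys pawn and weapon.
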(event Custom|Multicast_PlayWeaponSwing
  ;[1 1 1] Weapon Attack
  (bind _swingcurve (Timeline|Timeline PlayFromStart)
    (:Update
      (Transformation|SetRelativeRotation (Variables|Default|GetWeaponAttachmentPoint) (Math|Rotator|Lerp(Rotator) "0, 0, 0" "-90.000000,0.000000,0.000000" _swingcurve) false false)
      (Networking|SwitchHasAuthority
        (:Authority
          (CallFunction|EnableWeaponHitbox))))
    (:Finished
      (Variables|Default|SetSwingOnCooldown false)
      (CallFunction|DisableWeaponHitbox)
      (Class|BPIWeapon|ClearHitActors(Message) (Variables|Default|GetCurrentWeapon)))))

(event Custom|Server_KillPlayer
  (CallFunction|MulticastRagdoll)
  (Input|DisableInput 0)
  (Utilities|FlowControl|Delay 3.0)
  (bind _asbp_y2p_player_controller (Utilities|Casting|CastToBP_Y2P_PlayerController (Components|GetOwner (Variables|GetPlayerState)))
    (:then
      (Default|RespawnPlayer _asbp_y2p_player_controller)
      (Actor|DestroyActor (Variables|Default|GetCurrentWeapon))
      (Actor|DestroyActor))
    (:CastFailed
      (Development|PrintString "Failed Cast"))))

(event Custom|Multicast_SetTeamColor
  (params (TeamName :type Name))
  (switch name TeamName
    (:Red%20Team
      (Rendering|Material|SetMaterial (Variables|Default|GetArmor) 0 "/Game/Y2PrepHNSContent/Materials/Red.Red")
      (Rendering|Material|SetMaterial (Variables|Default|GetLEye) 0 "/Game/Y2PrepHNSContent/Materials/Red.Red")
      (Rendering|Material|SetMaterial (Variables|Default|GetREye) 0 "/Game/Y2PrepHNSContent/Materials/Red.Red"))
    (:Blue%20Team
      (Rendering|Material|SetMaterial (Variables|Default|GetArmor) 0 "/Game/Y2PrepHNSContent/Materials/Blue.Blue")
      (Rendering|Material|SetMaterial (Variables|Default|GetLEye) 0 "/Game/Y2PrepHNSContent/Materials/Blue.Blue")
      (Rendering|Material|SetMaterial (Variables|Default|GetREye) 0 "/Game/Y2PrepHNSContent/Materials/Blue.Blue"))))

(event Custom|Server_WeaponSwing
  ;[1 1 1] Weapon Attack
  (CallFunction|MulticastPlayWeaponSwing))

(event Custom|Multicast_Ragdoll
  (bind _body (Variables|Default|GetBody))
  (Physics|SetSimulatePhysics _body true)
  (Collision|SetCollisionEnabled _body "PhysicsOnly"))

(event Input|EnhancedActionEvents|EnhancedInputActionIA_Y2P_Attack
  (params (ActionValue :type Boolean) (ElapsedSeconds :type Float%20%28double-precision%29) (TriggeredSeconds :type Float%20%28double-precision%29) (InputAction :type Input%20Action%20Object%20Reference :default "/Game/Y2PrepHNSContent/Input/IA_Y2P_Attack.IA_Y2P_Attack"))
  ;[1 1 1] Weapon Attack
  (if (not (Variables|Default|GetSwingOnCooldown))
    (Variables|Default|SetSwingOnCooldown true)
    (CallFunction|ServerWeaponSwing)))

(event EventTakeDamage
  (params (DamageAmount :type Integer))
  (bind _asbp_y2p_player_state (Utilities|Casting|CastToBP_Y2P_PlayerState (Variables|GetPlayerState)))
  (if (<= (- (Variables|/Game/Y2PrepHNSContent/Framework/BP_Y2P_PlayerState.BP_Y2P_PlayerState_C|GetCurrentHealth _asbp_y2p_player_state) DamageAmount) (Variables|/Game/Y2PrepHNSContent/Framework/BP_Y2P_PlayerState.BP_Y2P_PlayerState_C|GetMaximumHealth _asbp_y2p_player_state))
    (bind _output_get (Variables|/Game/Y2PrepHNSContent/Framework/BP_Y2P_PlayerState.BP_Y2P_PlayerState_C|SetCurrentHealth _asbp_y2p_player_state (- (Variables|/Game/Y2PrepHNSContent/Framework/BP_Y2P_PlayerState.BP_Y2P_PlayerState_C|GetCurrentHealth _asbp_y2p_player_state) DamageAmount)))
    (if (<= _output_get 0)
      (CallFunction|ServerKillPlayer))))

(event EventBeginPlay
  (bind _asbp_y2p_player_controller (Utilities|Casting|CastToBP_Y2P_PlayerController (Pawn|GetController))
    (:then
      (Variables|Default|SetCachedController _asbp_y2p_player_controller))
    (:CastFailed
      (Development|PrintString "Hello"))))

(fn ConstructionScript)

(fn LoadClass
  (params (ClassData :type BP%20Y2P%20Class%20Data%20Object%20Reference))
  (bind _returnvalue (Game|SpawnActorfromClass (Variables|/Game/Y2PrepHNSContent/DataAssets/BP_Y2P_ClassData.BP_Y2P_ClassData_C|GetPrimaryWeaponMesh ClassData) (Transformation|GetActorTransform) "Undefined" "MultiplyWithRoot" 0 0))
  (Transformation|AttachComponentToComponent _returnvalue (Variables|Default|GetWeaponAttachmentPoint) "None" "SnapToTarget" "SnapToTarget" "SnapToTarget" true)
  (Variables|Default|SetCurrentWeapon _returnvalue))

(fn EnableWeaponHitbox
  (if true
    (Collision|SetCollisionEnabled (Actor|GetComponentbyClass (Variables|Default|GetCurrentWeapon) "/Script/Engine.BoxComponent") "QueryOnly")))

(fn DisableWeaponHitbox
  (bind _currentweapon (Variables|Default|GetCurrentWeapon))
  (if (Utilities|IsValid _currentweapon)
    (Collision|SetCollisionEnabled (Actor|GetComponentbyClass _currentweapon "/Script/Engine.BoxComponent") "NoCollision")))

(fn GetCurrentHealth
  (return 0))

(fn GetDamage
  (bind _asbp_y2p_player_state (Utilities|Casting|CastToBP_Y2P_PlayerState (Variables|GetPlayerState)))
  (return (Variables|/Game/Y2PrepHNSContent/DataAssets/BP_Y2P_ClassData.BP_Y2P_ClassData_C|GetPrimaryDamage (Variables|/Game/Y2PrepHNSContent/Framework/BP_Y2P_PlayerState.BP_Y2P_PlayerState_C|GetSelectedClassData _asbp_y2p_player_state))))

(fn GetMaxHealth
  (bind _asbp_y2p_player_state (Utilities|Casting|CastToBP_Y2P_PlayerState (Variables|GetPlayerState)))
  (return (Variables|/Game/Y2PrepHNSContent/Framework/BP_Y2P_PlayerState.BP_Y2P_PlayerState_C|GetMaximumHealth _asbp_y2p_player_state)))