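; Player controller that handles class selection, character spawning, HUD creation and team assignment.
; On BeginPlay, the local controller opens the class selection widget with UI-only input and a visible cursor.
; Server events spawn and possess a character, always loading DA_Warrior regardless of the selected class and with no spawn location yet, or write the team to PlayerState.
; A client event creates and stores the HUD widget.
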(event Custom|Server_SpawnCharacterWithClass
  (params (SelectedClassData :type BP%20Y2P%20Class%20Data%20Object%20Reference))
  (bind _returnvalue (Game|SpawnActorfromClass "/Game/Y2PrepHNSContent/Framework/BP_Y2P_Character.BP_Y2P_Character_C" (Math|Transform|MakeTransform "0, 0, 0" "0, 0, 0" "1.000000,1.000000,1.000000") "Undefined" "MultiplyWithRoot" 0 0)) ; Need to grab spawn locations
  (Pawn|Possess _returnvalue)
  (bind _asbp_y2p_character (Utilities|Casting|CastToBP_Y2P_Character _returnvalue))
  (Default|LoadClass _asbp_y2p_character "/Game/Y2PrepHNSContent/DataAssets/DA_Warrior.DA_Warrior"))

(event Custom|Server_SetTeam
  (params (TeamName :type Name))
  (bind _asbp_y2p_player_state (Utilities|Casting|CastToBP_Y2P_PlayerState (Game|GetPlayerState 0)))
  (Variables|/Game/Y2PrepHNSContent/Framework/BP_Y2P_PlayerState.BP_Y2P_PlayerState_C|SetPlayerTeam _asbp_y2p_player_state TeamName))

(event Custom|Client_ShowHUD
  (bind _returnvalue (UserInterface|CreateWidget "/Game/Y2PrepHNSContent/UI/WBP_Y2P_HUD.WBP_Y2P_HUD_C"))
  (UserInterface|Viewport|AddtoViewport _returnvalue 0)
  (Variables|Default|SetCurrentHUD _returnvalue))

(event EventBeginPlay
  (if (Pawn|IsLocalPlayerController)
    (bind _returnvalue (UserInterface|CreateWidget "/Game/Y2PrepHNSContent/UI/WBP_ClassSelection.WBP_ClassSelection_C"))
    (UserInterface|Viewport|AddtoViewport _returnvalue 0)
    (Input|SetInputModeUIOnly self 0 "DoNotLock" false)
    (Variables|Default|SetbShowMouseCursor true)))

(fn ConstructionScript)