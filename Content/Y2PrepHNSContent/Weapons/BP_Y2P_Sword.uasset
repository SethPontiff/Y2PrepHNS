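; BP_Y2P_Sword is a melee weapon that deals fixed damage to BP_Y2P_Character actors it overlaps.
; Its hit box starts with collision disabled, and this graph never re-enables it.
; A HitActors list limits damage to one hit per actor until ClearHitActors empties it.
; The owner check compares the overlapped character's owner to that character, rather than using the sword's own owner.
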(event EventBeginPlay
  (Collision|SetCollisionEnabled (Variables|Default|GetWeaponHitBox) "NoCollision"))

(event EventClearHitActors
  (Utilities|Array|Clear (Variables|Default|GetHitActors)))

(event Collision|EventActorBeginOverlap
  (params (OtherActor :type Actor%20Object%20Reference))
  (bind _hitactors (Variables|Default|GetHitActors))
  (bind _asbp_y2p_character (Utilities|Casting|CastToBP_Y2P_Character OtherActor))
  (if (!= (Components|GetOwner _asbp_y2p_character) OtherActor)
    (if (not (Utilities|Array|ContainsItem _hitactors OtherActor))
      (Utilities|Array|Add _hitactors OtherActor)
      (Class|BPIDamageable|TakeDamage(Message) _asbp_y2p_character 10))))

(fn ConstructionScript)