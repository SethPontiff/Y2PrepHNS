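; Player character that handles movement, camera look, jumping and a cosmetic melee weapon swing for multiplayer play.
; Adds an Enhanced Input mapping context on BeginPlay to drive those actions.
; A server event loads class data, spawning its primary weapon actor and attaching it to WeaponAttachmentPoint.
; Attacks route through server to multicast, where a timeline rotates that attachment point and clears the swing cooldown when finished.
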(event Custom|Server_LoadClass
  (params (ClassData :type BP%20Y2P%20Class%20Data%20Object%20Reference))
  (CallFunction|LoadClass ClassData))

(event Custom|Multicast_PlayWeaponSwing
  ;[1 1 1] Weapon Attack
  (bind _swingcurve (Timeline|WeaponSwing PlayFromStart)
    (:Update
      (Transformation|SetRelativeRotation (Variables|Default|GetWeaponAttachmentPoint) (Math|Rotator|Lerp(Rotator) "0, 0, 0" "-90.000000,0.000000,0.000000" _swingcurve) false false))
    (:Finished
      (Variables|Default|SetSwingOnCooldown false))))

(event Custom|Server_WeaponSwing
  ;[1 1 1] Weapon Attack
  (CallFunction|MulticastPlayWeaponSwing))

(event Input|EnhancedActionEvents|EnhancedInputActionIA_Y2P_Jump
  (params (ActionValue :type Boolean) (ElapsedSeconds :type Float%20%28double-precision%29) (TriggeredSeconds :type Float%20%28double-precision%29) (InputAction :type Input%20Action%20Object%20Reference :default "/Game/Y2PrepHNSContent/IA_Y2P_Jump.IA_Y2P_Jump"))
  ;[1 1 1] Jumping Logic
  (:Triggered
    (Character|Jump))
  (:Completed
    (Character|StopJumping)))

(event Input|EnhancedActionEvents|EnhancedInputActionIA_Y2P_Look
  (params (ActionValue :type Vector%202D%20Structure) (ElapsedSeconds :type Float%20%28double-precision%29) (TriggeredSeconds :type Float%20%28double-precision%29) (InputAction :type Input%20Action%20Object%20Reference :default "/Game/Y2PrepHNSContent/IA_Y2P_Look.IA_Y2P_Look"))
  ;[1 1 1] Camera
  (:Triggered
    (Pawn|Input|AddControllerYawInput (.x ActionValue))
    (Pawn|Input|AddControllerPitchInput (.y ActionValue))))

(event Input|EnhancedActionEvents|EnhancedInputActionIA_Y2P_Move
  (params (ActionValue :type Vector%202D%20Structure) (ElapsedSeconds :type Float%20%28double-precision%29) (TriggeredSeconds :type Float%20%28double-precision%29) (InputAction :type Input%20Action%20Object%20Reference :default "/Game/Y2PrepHNSContent/IA_Y2P_Move.IA_Y2P_Move"))
  (bind _returnvalue (Pawn|GetControlRotation :!class /Script/Engine.Pawn))
  ;[1 1 1] Movement Inputs
  (Pawn|Input|AddMovementInput (Math|Vector|GetRightVector (Math|Rotator|MakeRotator (.roll _returnvalue) 0.0 (.yaw _returnvalue))) (.x ActionValue) false)
  (Pawn|Input|AddMovementInput (Math|Vector|GetForwardVector (Math|Rotator|MakeRotator 0.0 0.0 (.yaw (Pawn|GetControlRotation :!class /Script/Engine.Pawn)))) (.y ActionValue) false))

(event Input|EnhancedActionEvents|EnhancedInputActionIA_Y2P_Attack
  (params (ActionValue :type Boolean) (ElapsedSeconds :type Float%20%28double-precision%29) (TriggeredSeconds :type Float%20%28double-precision%29) (InputAction :type Input%20Action%20Object%20Reference :default "/Game/Y2PrepHNSContent/IA_Y2P_Attack.IA_Y2P_Attack"))
  ;[1 1 1] Weapon Attack
  (if (not (Variables|Default|GetSwingOnCooldown))
    (Variables|Default|SetSwingOnCooldown true)
    (CallFunction|ServerWeaponSwing)))

(event EventBeginPlay
  ;[1 1 1] Grabbing Input Mapping At Start
  (Utilities|FlowControl|Sequence
    (:then_0
      (bind _asplayer_controller (Utilities|Casting|CastToPlayerController (Pawn|GetController)))
      (Utilities|IsValid (PlayerController|LocalPlayerSubsystems|GetEnhancedInputLocalPlayerSubsystem _asplayer_controller)
        (:Is%20Valid
          (Input|AddMappingContext (PlayerController|LocalPlayerSubsystems|GetEnhancedInputLocalPlayerSubsystem _asplayer_controller) "/Game/Y2PrepHNSContent/IMC_Y2P_Default.IMC_Y2P_Default" 0 "(bIgnoreAllPressedKeysUntilRelease=True,bForceImmediately=False,bNotifyUserSettings=False)"))))))

(fn ConstructionScript)

(fn LoadClass
  (params (ClassData :type BP%20Y2P%20Class%20Data%20Object%20Reference))
  (bind _returnvalue (Game|SpawnActorfromClass (Variables|/Game/Y2PrepHNSContent/BP_Y2P_ClassData.BP_Y2P_ClassData_C|GetPrimaryWeaponMesh ClassData) (Transformation|GetActorTransform) "Undefined" "MultiplyWithRoot" 0 0))
  (Transformation|AttachComponentToComponent _returnvalue (Variables|Default|GetWeaponAttachmentPoint) "None" "SnapToTarget" "SnapToTarget" "SnapToTarget" true))